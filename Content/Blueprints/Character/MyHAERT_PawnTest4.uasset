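; Test player pawn that fires a minigun and a flamethrower from primary or secondary weapon slots.
; Minigun uses a long line trace and flamethrower a shorter sphere trace, both debug-drawn, setting AutoDestroyWhenFinished on hit test enemies.
; Autofire events re-call themselves after a short delay while the matching slot's shooting flag is set.
; Trace ends use scaled camera-boom forward vectors without adding the actor's location.
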(event Custom|AutofireMinigun
  (bind (_outhit _returnvalue) (Collision|LineTraceForObjects (Transformation|GetActorLocation) (* (Math|Vector|GetForwardVector (Variables|Default|GetCameraBoom)) 5e+03) (Utilities|Array|MakeArray "ObjectTypeQuery3") false 0 "Persistent"))
  (if _returnvalue
    (bind _asmy_enemy_pawn_test_1 (Utilities|Casting|CastToMyEnemy_PawnTest1 (.HitActor (Collision|BreakHitResult _outhit)))
      (:then
        (Variables|/Script/Engine.Actor|SetbAutoDestroyWhenFinished _asmy_enemy_pawn_test_1 true))
      (:CastFailed
        _)))
  (switch Utilities|FlowControl|Switch|SwitchonEWeapons (Variables|Default|GetCurrentPrimaryWeapon)
    (:Minigun
      (if (Variables|Default|GetbIsShootingPrimary)
        (Utilities|FlowControl|Delay 0.2)
        (CallFunction|AutofireMinigun :!label _label)))
    (:FlameThrower
      (switch Utilities|FlowControl|Switch|SwitchonEWeapons (Variables|Default|GetCurrentSecondaryWeapon)
        (:Minigun
          (if (Variables|Default|GetbIsShootingSecondary)
            (Utilities|FlowControl|Delay 0.2)
            (goto _label)))))))

(event Custom|AutofireFlamethrower
  (bind (_outhit _returnvalue) (Collision|SphereTraceForObjects (Transformation|GetActorLocation) (* (Math|Vector|GetForwardVector (Variables|Default|GetCameraBoom)) 1e+03) 0.0 (Utilities|Array|MakeArray "ObjectTypeQuery3") false 0 "Persistent"))
  (if _returnvalue
    (bind _asmy_enemy_pawn_test_1 (Utilities|Casting|CastToMyEnemy_PawnTest1 (.HitActor (Collision|BreakHitResult _outhit)))
      (:then
        (Variables|/Script/Engine.Actor|SetbAutoDestroyWhenFinished _asmy_enemy_pawn_test_1 true))
      (:CastFailed
        _)))
  (switch Utilities|FlowControl|Switch|SwitchonEWeapons (Variables|Default|GetCurrentPrimaryWeapon)
    (:Minigun
      (switch Utilities|FlowControl|Switch|SwitchonEWeapons (Variables|Default|GetCurrentSecondaryWeapon)
        (:FlameThrower
          (if (Variables|Default|GetbIsShootingSecondary)
            (Utilities|FlowControl|Delay 0.2)
            (CallFunction|AutofireFlamethrower :!label _label)))))
    (:FlameThrower
      (if (Variables|Default|GetbIsShootingPrimary)
        (Utilities|FlowControl|Delay 0.2)
        (goto _label)))))

(event EventBeginPlay)

(event EventFireFlamethrower
  (Development|PrintString "fire")
  (bind (_outhit _returnvalue) (Collision|SphereTraceForObjects (Transformation|GetActorLocation) (* (Math|Vector|GetForwardVector (Variables|Default|GetCameraBoom)) 1e+03) 0.0 (Utilities|Array|MakeArray "ObjectTypeQuery3") false 0 "Persistent"))
  (if _returnvalue
    (bind _asmy_enemy_pawn_test_1 (Utilities|Casting|CastToMyEnemy_PawnTest1 (.HitActor (Collision|BreakHitResult _outhit)))
      (:then
        (Variables|/Script/Engine.Actor|SetbAutoDestroyWhenFinished _asmy_enemy_pawn_test_1 true))
      (:CastFailed
        _)))
  (switch Utilities|FlowControl|Switch|SwitchonEWeapons (Variables|Default|GetCurrentPrimaryWeapon)
    (:Minigun
      (switch Utilities|FlowControl|Switch|SwitchonEWeapons (Variables|Default|GetCurrentSecondaryWeapon)
        (:FlameThrower
          (if (Variables|Default|GetbIsShootingSecondary)
            (Utilities|FlowControl|Delay 0.2)
            (CallFunction|AutofireFlamethrower :!label _label)))))
    (:FlameThrower
      (if (Variables|Default|GetbIsShootingPrimary)
        (Utilities|FlowControl|Delay 0.2)
        (goto _label)))))

(event EventFireMinigun
  (bind (_outhit _returnvalue) (Collision|LineTraceForObjects (Transformation|GetActorLocation) (* (Math|Vector|GetForwardVector (Variables|Default|GetCameraBoom)) 5e+03) (Utilities|Array|MakeArray "ObjectTypeQuery3") false 0 "Persistent"))
  (if _returnvalue
    (bind _asmy_enemy_pawn_test_1 (Utilities|Casting|CastToMyEnemy_PawnTest1 (.HitActor (Collision|BreakHitResult _outhit)))
      (:then
        (Variables|/Script/Engine.Actor|SetbAutoDestroyWhenFinished _asmy_enemy_pawn_test_1 true))
      (:CastFailed
        _)))
  (switch Utilities|FlowControl|Switch|SwitchonEWeapons (Variables|Default|GetCurrentPrimaryWeapon)
    (:Minigun
      (if (Variables|Default|GetbIsShootingPrimary)
        (Utilities|FlowControl|Delay 0.2)
        (CallFunction|AutofireMinigun :!label _label)))
    (:FlameThrower
      (switch Utilities|FlowControl|Switch|SwitchonEWeapons (Variables|Default|GetCurrentSecondaryWeapon)
        (:Minigun
          (if (Variables|Default|GetbIsShootingSecondary)
            (Utilities|FlowControl|Delay 0.2)
            (goto _label)))))))

(fn ConstructionScript)