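; Test player pawn for a transforming vehicle that switches between biped and drive modes, each with normal and boosted speeds.
; Tick turns the upper body with the camera boom in biped mode or the mesh when driving, while two point lights blink alternately.
; Fire inputs trigger primary and secondary calls; weapon events use debug-drawn traces for minigun and flamethrower, and spawn dummy grenades.
; Minigun hits do nothing yet; flamethrower hits flag enemies for auto-destroy.
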(event Custom|AutofireMinigun
  (bind (_outhit _returnvalue) (Collision|LineTraceForObjects (Transformation|GetActorLocation) (* (Math|Vector|GetForwardVector (Variables|Default|GetCameraBoom)) 5e+03) (Utilities|Array|MakeArray "ObjectTypeQuery3") false 0 "Persistent"))
  (if _returnvalue
    _))

(event Custom|AutofireFlamethrower
  (bind (_outhit _returnvalue) (Collision|SphereTraceForObjects (Transformation|GetActorLocation) (* (Math|Vector|GetForwardVector (Variables|Default|GetCameraBoom)) 1e+03) 0.0 (Utilities|Array|MakeArray "ObjectTypeQuery3") false 0 "Persistent"))
  (if _returnvalue
    (bind _asmy_enemy_pawn_test_1 (Utilities|Casting|CastToMyEnemy_PawnTest1 (.HitActor (Collision|BreakHitResult _outhit))))
    (Variables|/Script/Engine.Actor|SetbAutoDestroyWhenFinished _asmy_enemy_pawn_test_1 true)))

(event EventFireGrenade
  (bind _returnvalue (Transformation|GetActorTransform))
  (bind (_location _rotation _scale) (Math|Transform|BreakTransform _returnvalue))
  (bind (_x _y _z) (Math|Vector|BreakVector _location))
  (Game|SpawnActorfromClass "/Game/Blueprints/ThirdPersonStrafeBP/Blueprints/DummyProjectile.DummyProjectile_C" (Math|Transform|MakeTransform (Math|Vector|MakeVector (+ _x 12.0) _y _z) _rotation _scale) "Undefined" 0 0))

(event EventBeginPlay
  (bind _pointlight (Variables|Default|GetPointLight))
  (bind _pointlight1 (Variables|Default|GetPointLight1))
  (Class|HAERTPawn|ChangeWeapons "Minigun" "FlameThrower")
  (Variables|Default|Setmy%20original (Variables|/Script/Engine.SceneComponent|GetRelativeLocation (Variables|Default|GetUpper)))
  (Utilities|FlowControl|Sequence
    (:then_0
      (Variables|Default|SetIntensity%202 (Variables|/Script/Engine.LightComponentBase|GetIntensity _pointlight1))
      (Utilities|FlowControl|Delay 0.2 :!label _label)
      (Rendering|Components|Light|SetIntensity _pointlight1 0.0)
      (Utilities|FlowControl|Delay 0.2)
      (Rendering|Components|Light|SetIntensity _pointlight1 (Variables|Default|GetIntensity%202))
      (goto _label))
    (:then_1
      (Variables|Default|SetIntensity1 (Variables|/Script/Engine.LightComponentBase|GetIntensity _pointlight))
      (Utilities|FlowControl|Delay 0.2 :!label _label_2)
      (Rendering|Components|Light|SetIntensity _pointlight (Variables|Default|GetIntensity1))
      (Utilities|FlowControl|Delay 0.2)
      (Rendering|Components|Light|SetIntensity _pointlight 0.0)
      (goto _label_2))))

(event EventFireFlamethrower
  (Development|PrintString "fire")
  (bind (_outhit _returnvalue) (Collision|SphereTraceForObjects (Transformation|GetActorLocation) (* (Math|Vector|GetForwardVector (Variables|Default|GetCameraBoom)) 1e+03) 0.0 (Utilities|Array|MakeArray "ObjectTypeQuery3") false 0 "Persistent"))
  (if _returnvalue
    (bind _asmy_enemy_pawn_test_1 (Utilities|Casting|CastToMyEnemy_PawnTest1 (.HitActor (Collision|BreakHitResult _outhit))))
    (Variables|/Script/Engine.Actor|SetbAutoDestroyWhenFinished _asmy_enemy_pawn_test_1 true)))

(event EventTick
  (params (DeltaSeconds :type Float%20%28single-precision%29))
  (bind _my_original (Variables|Default|Getmy%20original))
  (bind _upper (Variables|Default|GetUpper))
  (bind _relativerotation (Variables|/Script/Engine.SceneComponent|GetRelativeRotation _upper))
  (if (Variables|Default|GetBipedmode)
    (Transformation|SetRelativeRotation _upper (Math|Rotator|MakeRotator (.roll _relativerotation) (.pitch _relativerotation) (.yaw (Variables|/Script/Engine.SceneComponent|GetRelativeRotation (Variables|Default|GetCameraBoom)))) false false)
    (Transformation|SetRelativeLocation _upper (Variables|Default|Getmy%20original) false false)
    (Utilities|FlowControl|DoOnce false :!label _label
      (:Completed
        (goto _label_2 Reset)))
    (else
      (Transformation|SetRelativeRotation _upper (Math|Rotator|MakeRotator (.roll _relativerotation) (.pitch _relativerotation) (+ (.yaw (Variables|/Script/Engine.SceneComponent|GetRelativeRotation (Variables|Character|GetMesh))) 9e+01)) false false)
      (Utilities|FlowControl|DoOnce false :!label _label_2
        (:Completed
          (Transformation|SetRelativeLocation _upper (Math|Vector|MakeVector (.x _my_original) (.y _my_original) (+ (.z _my_original) 2.0)) false false)
          (goto _label Reset))))))

(event EventFireMinigun
  (bind (_outhit _returnvalue) (Collision|LineTraceForObjects (Transformation|GetActorLocation) (* (Math|Vector|GetForwardVector (Variables|Default|GetCameraBoom)) 5e+03) (Utilities|Array|MakeArray "ObjectTypeQuery3") false 0 "Persistent"))
  (if _returnvalue
    _))

(event Input|ActionEvents|InputActionAccelerate
  (params (Key :type Key%20Structure :default "AnyKey"))
  (bind _bipedmode (Variables|Default|GetBipedmode))
  (bind _charactermovement (Variables|Character|GetCharacterMovement))
  (:Pressed
    (if _bipedmode
      (Variables|/Script/Engine.CharacterMovementComponent|SetMaxWalkSpeed _charactermovement (Variables|Default|GetRunSpeed))
      (else
        (Variables|/Script/Engine.CharacterMovementComponent|SetMaxWalkSpeed _charactermovement (Variables|Default|GetDriveBoost)))))
  (:Released
    (if _bipedmode
      (Variables|/Script/Engine.CharacterMovementComponent|SetMaxWalkSpeed _charactermovement (Variables|Default|GetWalkspeed))
      (else
        (Variables|/Script/Engine.CharacterMovementComponent|SetMaxWalkSpeed _charactermovement (Variables|Default|GetDriveSpeed))))))

(event Input|ActionEvents|InputActionFirePrimary
  (params (Key :type Key%20Structure :default "AnyKey"))
  (:Pressed
    (Default|CallFAlpha)))

(event Input|ActionEvents|InputActionFireSecondary
  (params (Key :type Key%20Structure :default "AnyKey"))
  (:Pressed
    (Default|CallFBeta1)))

(event Input|ActionEvents|InputActionTransform
  (params (Key :type Key%20Structure :default "AnyKey"))
  (bind _charactermovement (Variables|Character|GetCharacterMovement))
  (:Pressed
    (if (Variables|Default|GetBipedmode)
      (Variables|Default|SetBipedmode false)
      (Variables|/Script/Engine.CharacterMovementComponent|SetMaxWalkSpeed _charactermovement (Variables|Default|GetDriveSpeed))
      (else
        (Variables|Default|SetBipedmode true)
        (Variables|/Script/Engine.CharacterMovementComponent|SetMaxWalkSpeed _charactermovement (Variables|Default|GetWalkspeed))))
    (Default|CallTransform)))

(fn ConstructionScript)